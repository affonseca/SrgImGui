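; Example Blueprint that shows how to set up an SRG ImGui Draw Tree node that draws a debug window.
; It registers under the SrgImGui.DrawTree tag on BeginPlay and unregisters on EndPlay.
; The node start callback opens a fixed-position window, draws a colored label and all info, then continues, or skips children if the window does not begin.
; The node end callback closes the window.
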(event EventBeginPlay
  (bind _returnvalue (Class|SrgImGuiSubsystem|Get)
    (:Valid
      (Class|SrgImGuiSubsystem|RegistertoDrawTree _returnvalue (Utilities|Set|MakeSet "(TagName=\"SrgImGui.DrawTree\")") "IgnoreWithWarning" "IgnoreWithWarning"))))

(event EventEndPlay
  (params (EndPlayReason :type EEndPlayReason%20Enum :default "Destroyed"))
  (bind _returnvalue (Class|SrgImGuiSubsystem|Get)
    (:Valid
      (Class|SrgImGuiSubsystem|UnregisterfromDrawTree _returnvalue))))

(fn ConstructionScript)

(fn DrawSrgImGuiInfo
  (params (SrgImGuiSubsystem :type Srg%20Im%20Gui%20Subsystem%20Object%20Reference)))

(fn ImGuiDrawTreeNodeEnd
  (params (NodeTag :type Gameplay%20Tag%20Structure%20%28by%20ref%29))
  (Class|SrgImGuiCoreLibrary|EndWindow)
  (return))

(fn ImGuiDrawTreeNodeStart
  (params (NodeTag :type Gameplay%20Tag%20Structure%20%28by%20ref%29))
  (Class|SrgImGuiCoreLibrary|SetNextWindowPosition "(X=20.000000,Y=20.000000)")
  (Class|SrgImGuiCoreLibrary|SetNextWindowSize "(X=600.000000,Y=750.000000)")
  (bind _returnvalue (Class|SrgImGuiCoreLibrary|BeginWindow "SRG ImGui Draw Tree Node Example" 17664))
  (if _returnvalue
    (Utilities|FlowControl|Sequence
      (:then_0
        (Class|SrgImGuiCoreLibrary|TextColored "This is an example of how to setup an SRG ImGui Draw Tree Node in BP." "(R=0.252778,G=0.230999,B=1.000000,A=1.000000)")
        (Class|SrgImGuiInfoLibrary|DrawAllInfo))
      (:then_1
        (return "Continue")))
    (else
      (return "SkipChildren"))))