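; Example Blueprint for the SRG ImGui plugin that draws a demo window through the Custom Drawer interface.
; The Draw function splits the window into collapsing headers for typed variable drawing, the default drawer and core ImGui features.
; DrawTypes lazily constructs a sample object and displays primitive, text, enum, class and container variables.
; DrawCoreImGui fans out to per-feature demo functions, including one showing how PushId/PopId scopes prevent duplicate-label bugs.
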(fn DrawTypes
  (Utilities|FlowControl|Sequence
    (:then_0
      (Utilities|IsValid (Variables|Default|GetObjectVariable)
        (:Is%20Not%20Valid
          (bind _returnvalue (Game|ConstructObjectfromClass "/SrgImGui/BP_SrgImGui_SimpleObject.BP_SrgImGui_SimpleObject_C"))
          (Variables|Default|SetObjectVariable _returnvalue))))
    (:then_1
      (Utilities|FlowControl|Sequence
        (:then_0
          ;[1 1 1] Primitive Variables
          (Class|SrgImGuiTypeLibrary|DrawBool "Bool Variable" (Variables|Default|GetBoolVariable) false)
          (Class|SrgImGuiTypeLibrary|DrawUInt8 "Byte Variable" (Variables|Default|GetByteVariable) false)
          (Class|SrgImGuiTypeLibrary|DrawInt32 "Integer Variable" (Variables|Default|GetIntegerVariable) false)
          (Class|SrgImGuiTypeLibrary|DrawInt64 "Integer 64 Variable" (Variables|Default|GetInteger64Variable) false)
          (Class|SrgImGuiTypeLibrary|DrawDouble "Float Variable" (Variables|Default|GetFloatVariable) false))
        (:then_1
          (Utilities|FlowControl|Sequence
            (:then_0
              ;[1 1 1] Text Variables
              (Class|SrgImGuiTypeLibrary|DrawName "Name Variable" (Variables|Default|GetNameVariable) false)
              (Class|SrgImGuiTypeLibrary|DrawString "String Variable" (Variables|Default|GetStringVariable) false)
              (Class|SrgImGuiTypeLibrary|DrawText "Text Variable" (Variables|Default|GetTextVariable) false))
            (:then_1
              (Utilities|FlowControl|Sequence
                (:then_0
                  ;[1 1 1] Enum Variable
                  (|K2NodeDrawEnum (Variables|Default|GetEnumVariable) "Enum Variable" false))
                (:then_1
                  (Utilities|FlowControl|Sequence
                    (:then_0
                      ;[1 1 1] Class Variables
                      (Class|SrgImGuiTypeLibrary|DrawClassK2Node "Class Variable" (Variables|Default|GetClassVariable) false)
                      (Class|SrgImGuiTypeLibrary|DrawSoftClassK2Node "Soft Class Variable" (Variables|Default|GetSoftClassVariable) false))
                    (:then_1
                      (Utilities|FlowControl|Sequence
                        (:then_0
                          ;[1 1 1] Container Variables
                          (Class|SrgImGuiTypeLibrary|DrawStructK2Node "Struct Variable" (Variables|Default|GetStructVariable) false true)
                          (Class|SrgImGuiTypeLibrary|DrawObject "Object Variable" (Variables|Default|GetObjectVariable) true)
                          (Class|SrgImGuiTypeLibrary|DrawArray "Array Variable" (Variables|Default|GetArrayVariable) false true)
                          (Class|SrgImGuiTypeLibrary|DrawSet "Set Variable" (Variables|Default|GetSetVariable) false true)
                          (Class|SrgImGuiTypeLibrary|DrawMap "Map Variable" (Variables|Default|GetMapVariable) false true))))))))))))))

(fn DrawCoreImGui
  (Utilities|FlowControl|Sequence
    (:then_0
      (bind _returnvalue (Class|SrgImGuiCoreLibrary|BeginTreeNode "Widgets"))
      (if _returnvalue
        (Utilities|FlowControl|Sequence
          (:then_0
            (bind _returnvalue_2 (Class|SrgImGuiCoreLibrary|BeginTreeNode "Basic"))
            (if _returnvalue_2
              (DrawCore|Widgets|DrawBasicWidgets)
              (Class|SrgImGuiCoreLibrary|EndTreeNode)))
          (:then_1
            (bind _returnvalue_3 (Class|SrgImGuiCoreLibrary|BeginTreeNode "Sliders"))
            (if _returnvalue_3
              (DrawCore|Widgets|DrawSliderWidgets)
              (Class|SrgImGuiCoreLibrary|EndTreeNode)))
          (:then_2
            (bind _returnvalue_4 (Class|SrgImGuiCoreLibrary|BeginTreeNode "Plots"))
            (if _returnvalue_4
              (DrawCore|Widgets|DrawPlotWidgets)
              (Class|SrgImGuiCoreLibrary|EndTreeNode)))
          (:then_3
            (Class|SrgImGuiCoreLibrary|EndTreeNode)))))
    (:then_1
      (Utilities|FlowControl|Sequence
        (:then_0
          (bind _returnvalue_5 (Class|SrgImGuiCoreLibrary|BeginTreeNode "Layout"))
          (if _returnvalue_5
            (DrawCore|DrawLayout)
            (Class|SrgImGuiCoreLibrary|EndTreeNode)))
        (:then_1
          (Utilities|FlowControl|Sequence
            (:then_0
              (bind _returnvalue_6 (Class|SrgImGuiCoreLibrary|BeginTreeNode "Windows"))
              (if _returnvalue_6
                (DrawCore|DrawWindow)
                (Class|SrgImGuiCoreLibrary|EndTreeNode)))
            (:then_1
              (Utilities|FlowControl|Sequence
                (:then_0
                  (bind _returnvalue_7 (Class|SrgImGuiCoreLibrary|BeginTreeNode "Menus"))
                  (if _returnvalue_7
                    (DrawCore|DrawMenus)
                    (Class|SrgImGuiCoreLibrary|EndTreeNode)))
                (:then_1
                  (Utilities|FlowControl|Sequence
                    (:then_0
                      (bind _returnvalue_8 (Class|SrgImGuiCoreLibrary|BeginTreeNode "Popups"))
                      (if _returnvalue_8
                        (DrawCore|DrawPopups)
                        (Class|SrgImGuiCoreLibrary|EndTreeNode)))
                    (:then_1
                      (Utilities|FlowControl|Sequence
                        (:then_0
                          (bind _returnvalue_9 (Class|SrgImGuiCoreLibrary|BeginTreeNode "Collapsing Header"))
                          (if _returnvalue_9
                            (DrawCore|DrawCollapsingHeader)
                            (Class|SrgImGuiCoreLibrary|EndTreeNode)))
                        (:then_1
                          (Utilities|FlowControl|Sequence
                            (:then_0
                              (bind _returnvalue_10 (Class|SrgImGuiCoreLibrary|BeginTreeNode "Tree"))
                              (if _returnvalue_10
                                (DrawCore|DrawTree)
                                (Class|SrgImGuiCoreLibrary|EndTreeNode)))
                            (:then_1
                              (Utilities|FlowControl|Sequence
                                (:then_0
                                  (bind _returnvalue_11 (Class|SrgImGuiCoreLibrary|BeginTreeNode "Tabs"))
                                  (if _returnvalue_11
                                    (DrawCore|DrawTabs)
                                    (Class|SrgImGuiCoreLibrary|EndTreeNode)))
                                (:then_1
                                  (Utilities|FlowControl|Sequence
                                    (:then_0
                                      (bind _returnvalue_12 (Class|SrgImGuiCoreLibrary|BeginTreeNode "Push and Pop Ids (IMPORTANT)"))
                                      (if _returnvalue_12
                                        (DrawCore|DrawPushPopId)
                                        (Class|SrgImGuiCoreLibrary|EndTreeNode)))))))))))))))))))))

(fn DrawBasicWidgets
  (Utilities|FlowControl|Sequence
    (:then_0
      (Class|SrgImGuiCoreLibrary|TextColored "This is colored text!" "(R=0.129974,G=0.757854,B=1.000000,A=1.000000)")
      (Class|SrgImGuiCoreLibrary|TextWrapped "This is wrapped text. It doesn't matter how long the text is, it will wrap correctly around the window."))
    (:then_1
      (Utilities|FlowControl|Sequence
        (:then_0
          (bind _returnvalue (Class|SrgImGuiCoreLibrary|Button "Regular Button"))
          (if _returnvalue
            (Development|PrintString 0 "Regular Button Clicked.")))
        (:then_1
          (Utilities|FlowControl|Sequence
            (:then_0
              (Class|SrgImGuiCoreLibrary|SameLine)
              (bind _returnvalue_2 (Class|SrgImGuiCoreLibrary|SmallButton "Small Button"))
              (if _returnvalue_2
                (Development|PrintString 0 "Small Button Clicked.")))
            (:then_1
              (Utilities|FlowControl|Sequence
                (:then_0
                  (Class|SrgImGuiCoreLibrary|SameLine)
                  (bind _returnvalue_3 (Class|SrgImGuiCoreLibrary|ButtonColored "Colored Button" "(R=0.202129,G=0.671875,B=0.192630,A=1.000000)"))
                  (if _returnvalue_3
                    (Development|PrintString 0 "Colored Button Clicked.")))
                (:then_1
                  (Utilities|FlowControl|Sequence
                    (:then_0
                      (Class|SrgImGuiCoreLibrary|SameLine)
                      (bind _returnvalue_4 (Class|SrgImGuiCoreLibrary|SmallButtonColored "Small Colored Button" "(R=0.765625,G=0.246479,B=0.170091,A=1.000000)"))
                      (if _returnvalue_4
                        (Development|PrintString 0 "Small Colored Button Clicked.")))
                    (:then_1
                      (Utilities|FlowControl|Sequence
                        (:then_0
                          (Class|SrgImGuiCoreLibrary|Combo "A Combo Box" (Variables|Default|GetListAndComboBoxItems) (Variables|Default|GetListAndComboBoxSelectedItemIndex))
                          (Class|SrgImGuiCoreLibrary|List "A List Box" (Variables|Default|GetListAndComboBoxItems) (Variables|Default|GetListAndComboBoxSelectedItemIndex)))
                        (:then_1
                          (Utilities|FlowControl|Sequence
                            (:then_0
                              (Class|SrgImGuiCoreLibrary|ColorEdit "Color Edit" (Variables|Default|GetColor))
                              (Class|SrgImGuiCoreLibrary|LinearColorEdit "Linear Color Edit" (Variables|Default|GetLinearColor)))))))))))))))))

(fn DrawLayout
  (Utilities|FlowControl|Sequence
    (:then_0
      (bind _returnvalue (Class|SrgImGuiCoreLibrary|BeginTreeNode "Same Line"))
      (if _returnvalue
        (Class|SrgImGuiCoreLibrary|TextColored "\"Same Line\" can be used" "(R=0.000000,G=0.981460,B=1.000000,A=1.000000)")
        (Class|SrgImGuiCoreLibrary|SameLine)
        (Class|SrgImGuiCoreLibrary|TextColored "to have two widgets in the same line." "(R=1.000000,G=0.203286,B=0.143550,A=1.000000)")
        (Class|SrgImGuiCoreLibrary|EndTreeNode)))
    (:then_1
      (Utilities|FlowControl|Sequence
        (:then_0
          (bind _returnvalue_2 (Class|SrgImGuiCoreLibrary|BeginTreeNode "New Line"))
          (if _returnvalue_2
            (Class|SrgImGuiCoreLibrary|TextColored "\"New Line\" can be used" "(R=0.000000,G=0.981460,B=1.000000,A=1.000000)")
            (Class|SrgImGuiCoreLibrary|NewLine)
            (Class|SrgImGuiCoreLibrary|TextColored "to create empy lines." "(R=1.000000,G=0.203286,B=0.143550,A=1.000000)")
            (Class|SrgImGuiCoreLibrary|EndTreeNode)))
        (:then_1
          (Utilities|FlowControl|Sequence
            (:then_0
              (bind _returnvalue_3 (Class|SrgImGuiCoreLibrary|BeginTreeNode "Spacing"))
              (if _returnvalue_3
                (Class|SrgImGuiCoreLibrary|TextColored "\"Spacing\" can be used for the same effect as \"New Line\"" "(R=0.000000,G=0.981460,B=1.000000,A=1.000000)")
                (Class|SrgImGuiCoreLibrary|Spacing)
                (Class|SrgImGuiCoreLibrary|TextColored "but the effect is more subtle." "(R=1.000000,G=0.203286,B=0.143550,A=1.000000)")
                (Class|SrgImGuiCoreLibrary|EndTreeNode)))
            (:then_1
              (Utilities|FlowControl|Sequence
                (:then_0
                  (bind _returnvalue_4 (Class|SrgImGuiCoreLibrary|BeginTreeNode "Dummy"))
                  (if _returnvalue_4
                    (Class|SrgImGuiCoreLibrary|TextColored "To add custom padding between elements, " "(R=0.000000,G=0.981460,B=1.000000,A=1.000000)")
                    (Class|SrgImGuiCoreLibrary|SameLine)
                    (Class|SrgImGuiCoreLibrary|Dummy "(X=100.000000,Y=10.000000)")
                    (Class|SrgImGuiCoreLibrary|SameLine)
                    (Class|SrgImGuiCoreLibrary|TextColored "\"Dummy\" can be used." "(R=1.000000,G=0.203286,B=0.143550,A=1.000000)")
                    (Class|SrgImGuiCoreLibrary|EndTreeNode)))
                (:then_1
                  (Utilities|FlowControl|Sequence
                    (:then_0
                      (bind _returnvalue_5 (Class|SrgImGuiCoreLibrary|BeginTreeNode "Separator"))
                      (if _returnvalue_5
                        (Class|SrgImGuiCoreLibrary|TextColored "This is a \"Separator\"" "(R=0.000000,G=0.981460,B=1.000000,A=1.000000)")
                        (Class|SrgImGuiCoreLibrary|Separator)
                        (Class|SrgImGuiCoreLibrary|TextColored "between widgets." "(R=1.000000,G=0.203286,B=0.143550,A=1.000000)")
                        (Class|SrgImGuiCoreLibrary|EndTreeNode)))
                    (:then_1
                      (Utilities|FlowControl|Sequence
                        (:then_0
                          (bind _returnvalue_6 (Class|SrgImGuiCoreLibrary|BeginTreeNode "Set Next Item Width"))
                          (if _returnvalue_6
                            (Class|SrgImGuiCoreLibrary|TextWrapped "Some widgets can have their size modified by \"Set Next Item Width\":")
                            (Class|SrgImGuiCoreLibrary|SetNextItemWidth 2e+01)
                            (Class|SrgImGuiCoreLibrary|Combo "Tiny Combo Box" (Variables|Default|GetListAndComboBoxItems) (Variables|Default|GetListAndComboBoxSelectedItemIndex))
                            (Class|SrgImGuiCoreLibrary|EndTreeNode)))
                        (:then_1
                          (Utilities|FlowControl|Sequence
                            (:then_0
                              (bind _returnvalue_7 (Class|SrgImGuiCoreLibrary|BeginTreeNode "Indent"))
                              (if _returnvalue_7
                                (Class|SrgImGuiCoreLibrary|TextColored "Widgets" "(R=0.396078,G=1.000000,B=0.501961,A=1.000000)")
                                (Class|SrgImGuiCoreLibrary|Indent 0.0)
                                (Class|SrgImGuiCoreLibrary|TextColored "can be" "(R=0.396078,G=1.000000,B=0.501961,A=1.000000)")
                                (Class|SrgImGuiCoreLibrary|Indent 0.0)
                                (Class|SrgImGuiCoreLibrary|TextColored "indented." "(R=0.396078,G=1.000000,B=0.501961,A=1.000000)")
                                (Class|SrgImGuiCoreLibrary|Unindent 0.0)
                                (Class|SrgImGuiCoreLibrary|TextColored "But they" "(R=0.396078,G=1.000000,B=0.501961,A=1.000000)")
                                (Class|SrgImGuiCoreLibrary|Unindent 0.0)
                                (Class|SrgImGuiCoreLibrary|TextColored "can also be" "(R=0.396078,G=1.000000,B=0.501961,A=1.000000)")
                                (Class|SrgImGuiCoreLibrary|Unindent 0.0)
                                (Class|SrgImGuiCoreLibrary|TextColored "unindented." "(R=0.396078,G=1.000000,B=0.501961,A=1.000000)")
                                (Class|SrgImGuiCoreLibrary|EndTreeNode)))
                            (:then_1
                              (Utilities|FlowControl|Sequence
                                (:then_0
                                  (bind _returnvalue_8 (Class|SrgImGuiCoreLibrary|BeginTreeNode "Columns"))
                                  (if _returnvalue_8
                                    (Class|SrgImGuiCoreLibrary|TextColored "Columns can be used to create tables:" "(R=0.000000,G=0.981460,B=1.000000,A=1.000000)")
                                    (Class|SrgImGuiCoreLibrary|BeginColumns "Colums Example" 2)
                                    (Class|SrgImGuiCoreLibrary|TextColored "Vegetables" "(R=0.446675,G=1.000000,B=0.408355,A=1.000000)")
                                    (Class|SrgImGuiCoreLibrary|TextWrapped "Carrot")
                                    (Class|SrgImGuiCoreLibrary|TextWrapped "Lettuce")
                                    (Class|SrgImGuiCoreLibrary|TextWrapped "Cabbage")
                                    (Class|SrgImGuiCoreLibrary|NextColumn)
                                    (Class|SrgImGuiCoreLibrary|TextColored "Fruits" "(R=1.000000,G=0.124469,B=0.114522,A=1.000000)")
                                    (Class|SrgImGuiCoreLibrary|TextWrapped "Apple")
                                    (Class|SrgImGuiCoreLibrary|TextWrapped "Banana")
                                    (Class|SrgImGuiCoreLibrary|TextWrapped "Pear")
                                    (Class|SrgImGuiCoreLibrary|EndColumns)
                                    (Class|SrgImGuiCoreLibrary|EndTreeNode)))))))))))))))))))

(fn DrawWindow
  (Class|SrgImGuiTypeLibrary|DrawBool "Show Closable Window" (Variables|Default|GetDrawClosableWindow) true)
  (if (Variables|Default|GetDrawClosableWindow)
    (Class|SrgImGuiCoreLibrary|SetNextWindowSize "(X=200.000000,Y=100.000000)")
    (Class|SrgImGuiCoreLibrary|SetNextWindowPosition "(X=950.000000,Y=900.000000)")
    (bind _returnvalue (Class|SrgImGuiCoreLibrary|BeginClosableWindow "A closable window" 0 (Variables|Default|GetDrawClosableWindow)))
    (if _returnvalue
      (Class|SrgImGuiCoreLibrary|TextColored "This is a new closable window!" "(R=1.000000,G=0.008226,B=0.900370,A=1.000000)"))
    (Class|SrgImGuiCoreLibrary|EndWindow)))

(fn DrawMenus
  (Class|SrgImGuiCoreLibrary|TextWrapped "Menus are displayed at the top of the window. Look for \"The First Menu\" and \"The Second Menu (Disabled)\".")
  (bind _returnvalue (Class|SrgImGuiCoreLibrary|BeginMenuBar))
  (if _returnvalue
    (Utilities|FlowControl|Sequence
      (:then_0
        (bind _returnvalue_2 (Class|SrgImGuiCoreLibrary|BeginMenu "The First Menu" true))
        (if _returnvalue_2
          (Utilities|FlowControl|Sequence
            (:then_0
              (bind _returnvalue_3 (Class|SrgImGuiCoreLibrary|BeginMenu "This is a submenu" true))
              (if _returnvalue_3
                (bind _returnvalue_4 (Class|SrgImGuiCoreLibrary|MenuItem "Submenu Item 1" true))
                (if _returnvalue_4
                  (Development|PrintString 0 "Submenu Item 1 Activated"))
                (bind _returnvalue_5 (Class|SrgImGuiCoreLibrary|MenuItem "Submenu Item 2" true))
                (if _returnvalue_5
                  (Development|PrintString 0 "Submenu Item 2 Activated"))
                (Class|SrgImGuiCoreLibrary|EndMenu)))
            (:then_1
              (bind _returnvalue_6 (Class|SrgImGuiCoreLibrary|MenuItem "Default Menu Item" true))
              (if _returnvalue_6
                (Development|PrintString 0 "Default Menu Item 1 Activated"))
              (Class|SrgImGuiCoreLibrary|SelectableMenuItem "Selectable Menu Item " (Variables|Default|GetMenuItemSelected) true)
              (Utilities|FlowControl|Sequence
                (:then_0
                  (if (Variables|Default|GetMenuItemSelected)
                    (Class|SrgImGuiCoreLibrary|MenuItem "Show based on Selectable Menu Item" true)))
                (:then_1
                  (Class|SrgImGuiCoreLibrary|MenuItem "Disabled Menu Item" false))))
            (:then_2
              (Class|SrgImGuiCoreLibrary|EndMenu)))))
      (:then_1
        (bind _returnvalue_7 (Class|SrgImGuiCoreLibrary|BeginMenu "The Second Menu (Disabled)" false))
        (if _returnvalue_7
          (Class|SrgImGuiCoreLibrary|EndMenu)))
      (:then_2
        (Class|SrgImGuiCoreLibrary|EndMenuBar)))))

(fn DrawPopups
  ;[1 1 1] Menu Popup
  (Utilities|FlowControl|Sequence
    (:then_0
      (bind _returnvalue (Class|SrgImGuiCoreLibrary|Button "Open Menu Popup"))
      (if _returnvalue
        (Class|SrgImGuiCoreLibrary|OpenPopup "Popup Menu"))
      (bind _returnvalue_2 (Class|SrgImGuiCoreLibrary|BeginPopupMenu "Popup Menu"))
      (if _returnvalue_2
        (Utilities|FlowControl|Sequence
          (:then_0
            (bind _returnvalue_3 (Class|SrgImGuiCoreLibrary|BeginMenu "Popup Submenu" true))
            (if _returnvalue_3
              (bind _returnvalue_4 (Class|SrgImGuiCoreLibrary|MenuItem "Popup Submenu Item 1" true))
              (if _returnvalue_4
                (Development|PrintString 0 "Popup Submenu Item 1 Activated"))
              (bind _returnvalue_5 (Class|SrgImGuiCoreLibrary|MenuItem "Popup Submenu Item 2" true))
              (if _returnvalue_5
                (Development|PrintString 0 "Popup Submenu Item 2 Activated"))
              (Class|SrgImGuiCoreLibrary|EndMenu)))
          (:then_1
            (bind _returnvalue_6 (Class|SrgImGuiCoreLibrary|MenuItem "Popup Menu Item" true))
            (if _returnvalue_6
              (Development|PrintString 0 "Popup Menu Item Activated")))
          (:then_2
            (Class|SrgImGuiCoreLibrary|EndPopup)))))
    (:then_1
      ;[1 1 1] Modal Popup
      (Utilities|FlowControl|Sequence
        (:then_0
          (bind _returnvalue_7 (Class|SrgImGuiCoreLibrary|Button "Open Modal Popup"))
          (if _returnvalue_7
            (Class|SrgImGuiCoreLibrary|OpenPopup "Popup Modal"))
          (bind _returnvalue_8 (Class|SrgImGuiCoreLibrary|BeginPopupModal "Popup Modal"))
          (if _returnvalue_8
            (Class|SrgImGuiCoreLibrary|TextColored "This is a Popup!" "(R=0.066385,G=0.151397,B=1.000000,A=1.000000)")
            (Class|SrgImGuiCoreLibrary|TextWrapped "It can only be closed with a call to \"Close Current Popup\".")
            (bind _returnvalue_9 (Class|SrgImGuiCoreLibrary|Button "Close"))
            (if _returnvalue_9
              (Class|SrgImGuiCoreLibrary|CloseCurrentPopup))
            (Class|SrgImGuiCoreLibrary|EndPopup)))
        (:then_1
          ;[1 1 1] Closable Menu Popup
          (Utilities|FlowControl|Sequence
            (:then_0
              (bind _returnvalue_10 (Class|SrgImGuiCoreLibrary|Button "Open Closable Modal Popup"))
              (if _returnvalue_10
                (Class|SrgImGuiCoreLibrary|OpenPopup "Closable Popup Modal"))
              (bind _returnvalue_11 (Class|SrgImGuiCoreLibrary|BeginClosablePopupModal "Closable Popup Modal"))
              (if _returnvalue_11
                (Class|SrgImGuiCoreLibrary|TextColored "This is a closabled Popup!" "(R=1.000000,G=0.072683,B=0.873928,A=1.000000)")
                (Class|SrgImGuiCoreLibrary|EndPopup)))))))))

(fn DrawCollapsingHeader
  (bind _returnvalue (Class|SrgImGuiCoreLibrary|CollapsingHeader "A Collapsing Header"))
  (if _returnvalue
    (Class|SrgImGuiCoreLibrary|TextColored "This is the content of a collapsing header." "(R=1.000000,G=0.092579,B=0.072683,A=1.000000)"))
  (Class|SrgImGuiTypeLibrary|DrawBool "Show Closable Collapsing Header" (Variables|Default|GetDrawClosableCollapsingHeader) true)
  (bind _returnvalue_2 (Class|SrgImGuiCoreLibrary|ClosableCollapsingHeader "A Closable Collapsing Header" (Variables|Default|GetDrawClosableCollapsingHeader)))
  (if _returnvalue_2
    (Class|SrgImGuiCoreLibrary|TextColored "This is the content of a closable collapsing header." "(R=0.249928,G=1.000000,B=0.345757,A=1.000000)")))

(fn DrawTree
  (Utilities|FlowControl|Sequence
    (:then_0
      (bind _returnvalue (Class|SrgImGuiCoreLibrary|BeginTreeNode "Node A"))
      (if _returnvalue
        (Class|SrgImGuiCoreLibrary|TextWrapped "This is node A.")
        (Utilities|FlowControl|Sequence
          (:then_0
            (bind _returnvalue_2 (Class|SrgImGuiCoreLibrary|BeginTreeNode "Node A.1"))
            (if _returnvalue_2
              (Class|SrgImGuiCoreLibrary|TextWrapped "This is node A.1")
              (Class|SrgImGuiCoreLibrary|EndTreeNode)))
          (:then_1
            (bind _returnvalue_3 (Class|SrgImGuiCoreLibrary|BeginTreeNode "Node A.2"))
            (if _returnvalue_3
              (Class|SrgImGuiCoreLibrary|TextWrapped "This is node A.2")
              (Class|SrgImGuiCoreLibrary|EndTreeNode)))
          (:then_2
            (Class|SrgImGuiCoreLibrary|EndTreeNode)))))
    (:then_1
      (Utilities|FlowControl|Sequence
        (:then_0
          (bind _returnvalue_4 (Class|SrgImGuiCoreLibrary|BeginTreeNode "Node B"))
          (if _returnvalue_4
            (Class|SrgImGuiCoreLibrary|TextWrapped "This is node B.")
            (Utilities|FlowControl|Sequence
              (:then_0
                (bind _returnvalue_5 (Class|SrgImGuiCoreLibrary|BeginTreeNode "Node B.1"))
                (if _returnvalue_5
                  (Class|SrgImGuiCoreLibrary|TextWrapped "This is node B.1")
                  (Class|SrgImGuiCoreLibrary|EndTreeNode)))
              (:then_1
                (Class|SrgImGuiCoreLibrary|EndTreeNode)))))))))

(fn DrawTabs
  (Class|SrgImGuiTypeLibrary|DrawBool "Show Closable Tab" (Variables|Default|GetDrawClosableTab) true)
  (bind _returnvalue (Class|SrgImGuiCoreLibrary|BeginTabBar "A Tab Bar"))
  (if _returnvalue
    (Utilities|FlowControl|Sequence
      (:then_0
        (bind _returnvalue_2 (Class|SrgImGuiCoreLibrary|BeginTab "First Tab"))
        (if _returnvalue_2
          (Class|SrgImGuiCoreLibrary|TextColored "This is the content of the first tab." "(R=0.936053,G=0.193868,B=1.000000,A=1.000000)")
          (Class|SrgImGuiCoreLibrary|EndTab)))
      (:then_1
        (bind _returnvalue_3 (Class|SrgImGuiCoreLibrary|BeginTab "Second Tab"))
        (if _returnvalue_3
          (Class|SrgImGuiCoreLibrary|TextColored "This is the content of the second tab." "(R=1.000000,G=0.912296,B=0.112380,A=1.000000)")
          (Class|SrgImGuiCoreLibrary|EndTab)))
      (:then_2
        (bind _returnvalue_4 (Class|SrgImGuiCoreLibrary|BeginClosableTab "Closable Tab" (Variables|Default|GetDrawClosableTab)))
        (if _returnvalue_4
          (Class|SrgImGuiCoreLibrary|TextColored "This is the content of the closable tab." "(R=0.438970,G=1.000000,B=0.281627,A=1.000000)")
          (Class|SrgImGuiCoreLibrary|EndTab)))
      (:then_3
        (Class|SrgImGuiCoreLibrary|EndTabBar)))))

(fn DrawPushPopId
  (Utilities|FlowControl|Sequence
    (:then_0
      (Class|SrgImGuiCoreLibrary|TextWrapped "Understanding how ids work is very important to avoid bugs when working with ImGui.")
      (Class|SrgImGuiCoreLibrary|TextWrapped "Most items that are added through ImGui have a \"label\" or \"id\" parameter that identifies that specific item.")
      (Class|SrgImGuiCoreLibrary|TextWrapped "As such, it's important that no two items of the same type share the same label/id.")
      (Class|SrgImGuiCoreLibrary|TextWrapped "This is not always desirable, especially when iterating through a list."))
    (:then_1
      (Utilities|FlowControl|Sequence
        (:then_0
          (Class|SrgImGuiCoreLibrary|TextWrapped "That is why ImGui provides a \"Push Id \"and \"Pop Id\" functionality.")
          (Class|SrgImGuiCoreLibrary|TextWrapped "Pushing an id creates a new scope. Within it, all ids are isolated from the outside.")
          (Class|SrgImGuiCoreLibrary|TextWrapped "It's even possible to create scopes within scopes.")
          (Class|SrgImGuiCoreLibrary|TextWrapped "Always pair \"Push Id\" with \"Pop Id\" to close the scope."))
        (:then_1
          (Utilities|FlowControl|Sequence
            (:then_0
              (Class|SrgImGuiCoreLibrary|NewLine)
              (Class|SrgImGuiCoreLibrary|TextColored "This is an example of how using the same label or id can cause bugs:" "(R=1.000000,G=0.020309,B=0.010362,A=1.000000)")
              (bind _returnvalue (Class|SrgImGuiCoreLibrary|CollapsingHeader "Duplicated Label"))
              (if _returnvalue
                (Class|SrgImGuiCoreLibrary|TextColored "Inside Duplicated Label 1" "(R=1.000000,G=0.969105,B=0.138749,A=1.000000)"))
              (bind _returnvalue_2 (Class|SrgImGuiCoreLibrary|CollapsingHeader "Duplicated Label"))
              (if _returnvalue_2
                (Class|SrgImGuiCoreLibrary|TextColored "Inside Duplicated Label 2" "(R=0.184967,G=1.000000,B=0.304154,A=1.000000)")))
            (:then_1
              (Utilities|FlowControl|Sequence
                (:then_0
                  (Class|SrgImGuiCoreLibrary|NewLine)
                  (Class|SrgImGuiCoreLibrary|TextColored "This is how to fix the previous issue while keeping the same labels:" "(R=0.101385,G=1.000000,B=0.170446,A=1.000000)")
                  (Class|SrgImGuiCoreLibrary|PushId "Duplicated Label 1")
                  (bind _returnvalue_3 (Class|SrgImGuiCoreLibrary|CollapsingHeader "Duplicated Label"))
                  (if _returnvalue_3
                    (Class|SrgImGuiCoreLibrary|TextColored "Inside Duplicated Label 1" "(R=1.000000,G=0.969105,B=0.138749,A=1.000000)"))
                  (Class|SrgImGuiCoreLibrary|PopId)
                  (Class|SrgImGuiCoreLibrary|PushId "Duplicated Label 2")
                  (bind _returnvalue_4 (Class|SrgImGuiCoreLibrary|CollapsingHeader "Duplicated Label"))
                  (if _returnvalue_4
                    (Class|SrgImGuiCoreLibrary|TextColored "Inside Duplicated Label 2" "(R=0.184967,G=1.000000,B=0.304154,A=1.000000)"))
                  (Class|SrgImGuiCoreLibrary|PopId))
                (:then_1
                  (Utilities|FlowControl|Sequence
                    (:then_0
                      (Class|SrgImGuiCoreLibrary|NewLine)
                      (Class|SrgImGuiCoreLibrary|TextWrapped "SRG ImGui creates an id scope for both the \"Draw Tree\" and \"Custom Drawer\" interface functions.")
                      (Class|SrgImGuiCoreLibrary|TextWrapped "As such, each function is protected from clashing with ids from other objects.")
                      (Class|SrgImGuiCoreLibrary|TextWrapped "However, within the same interface, id duplication can still occur."))))))))))))

(fn DrawSliderWidgets
  (Class|SrgImGuiCoreLibrary|Uint8Slider "Byte Slider" (Variables|Default|GetByteVariable) 0 10)
  (Class|SrgImGuiCoreLibrary|Int32Slider "Integer Slider" (Variables|Default|GetIntegerVariable) 0 10)
  (Class|SrgImGuiCoreLibrary|Int64Slider "Integer 64 Slider" (Variables|Default|GetInteger64Variable) 0 10000)
  (Class|SrgImGuiCoreLibrary|DoubleSlider "Float Slider" (Variables|Default|GetFloatVariable) 0.0 1.0))

(fn DrawPlotWidgets
  (Class|SrgImGuiCoreLibrary|PlotHistogram "Plot Histogram" (Variables|Default|GetArrayVariable) "" "(X=500.000000,Y=75.000000)")
  (Class|SrgImGuiCoreLibrary|PlotHistogramClamped "Plot Histogram (Clamped)" (Variables|Default|GetArrayVariable) "Clamped between -10 and 10." "(X=500.000000,Y=75.000000)" -1e+01 1e+01)
  (Class|SrgImGuiCoreLibrary|PlotLines "Plot Lines" (Variables|Default|GetArrayVariable) "" "(X=500.000000,Y=75.000000)")
  (Class|SrgImGuiCoreLibrary|PlotLinesClamped "Plot Lines (Clamped)" (Variables|Default|GetArrayVariable) "Clamped between -10 and 10." "(X=500.000000,Y=75.000000)" -1e+01 1e+01))

(fn ImGuiCustomDrawerDraw
  (Utilities|FlowControl|Sequence
    (:then_0
      (Class|SrgImGuiCoreLibrary|SetNextWindowPosition "(X=700.000000,Y=20.000000)")
      (Class|SrgImGuiCoreLibrary|SetNextWindowSize "(X=700.000000,Y=750.000000)")
      (bind _returnvalue (Class|SrgImGuiCoreLibrary|BeginWindow "SRG ImGui Custom Drawer Demo" 17664))
      (if _returnvalue
        (Utilities|FlowControl|Sequence
          (:then_0
            (Class|SrgImGuiCoreLibrary|TextColored (Utilities|GetTitleString) "(R=0.047516,G=1.000000,B=0.222282,A=1.000000)")
            (Class|SrgImGuiCoreLibrary|TextWrapped "This Blueprint Class is an example of how to use the SRG ImGui Library Custom Drawer and Blueprint Library Functions.")
            (Class|SrgImGuiCoreLibrary|NewLine)
            (Class|SrgImGuiCoreLibrary|TextWrapped "Every function of the library is fully documented. Hovering with the mouse over the node should display a tooltip.")
            (Class|SrgImGuiCoreLibrary|TextWrapped "This is true even for parameters or return values."))
          (:then_1
            (Utilities|FlowControl|Sequence
              (:then_0
                (bind _returnvalue_2 (Class|SrgImGuiCoreLibrary|CollapsingHeader "Drawing Types"))
                (if _returnvalue_2
                  (Class|SrgImGuiCoreLibrary|Indent 0.0)
                  (CallFunction|DrawTypes)
                  (Class|SrgImGuiCoreLibrary|Unindent 0.0)))
              (:then_1
                (Utilities|FlowControl|Sequence
                  (:then_0
                    (bind _returnvalue_3 (Class|SrgImGuiCoreLibrary|CollapsingHeader "Default Drawer"))
                    (if _returnvalue_3
                      (Class|SrgImGuiCoreLibrary|Indent 0.0)
                      (Class|SrgImGuiTypeLibrary|DrawDefaultCustomDrawer "Default Drawer" false)
                      (Class|SrgImGuiCoreLibrary|Unindent 0.0)))
                  (:then_1
                    (Utilities|FlowControl|Sequence
                      (:then_0
                        (bind _returnvalue_4 (Class|SrgImGuiCoreLibrary|CollapsingHeader "Drawing Core ImGui"))
                        (if _returnvalue_4
                          (Class|SrgImGuiCoreLibrary|Indent 0.0)
                          (CallFunction|DrawCoreImGui)
                          (Class|SrgImGuiCoreLibrary|Unindent 0.0))))))))))))
    (:then_1
      (Class|SrgImGuiCoreLibrary|EndWindow))))